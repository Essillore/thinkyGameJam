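; BP_MusicStones_B is the B-note music stone, tracking whether it is triggered as the third step of a note sequence.
; On any actor overlap it increments its note counter, then finds all BP_MusicStones_C actors.
; For each, it copies that stone's second-note flag into its own third-note flag, printing a debug message when true, so the last one checked decides.
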(event `self.ReceiveActorBeginOverlap`
  (params (OtherActor :type "Actor Object Reference"))
  (set `self.Note_B_count` (+ (`self.Note_B_count`) 1.0))
  (bind _outactors (`GameplayStatics.GetAllActorsOfClass` "/Game/BlueprintsMusicStones/BP_MusicStones_C.BP_MusicStones_C_C"))
  (for _array_element _outactors
    (bind _asbp_music_stones_c (cast `/Game/BlueprintsMusicStones/BP_MusicStones_C` _array_element))
    (if (`/Game/BlueprintsMusicStones/BP_MusicStones_C.Note_2_first` _asbp_music_stones_c)
      (set `self.Note_3_first` true)
      (`KismetSystemLibrary.PrintString` "3 first notes")
      (else
        (set `self.Note_3_first` false)))))

(fn `UserConstructionScript`)