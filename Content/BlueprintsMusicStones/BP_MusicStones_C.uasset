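; BP_MusicStones_C is an actor for the C note in a music stones mechanic, apparently unfinished.
; On BeginPlay it caches the music stones GameInstance, and each actor overlap increments a C note counter.
; A disconnected branch would read the GameInstance's NoteCPressed flag to set Note2First and print a debug message, but it never runs, and the counter's comparison is unused.
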(event `self.ReceiveBeginPlay`
  (bind _asbp_music_stones_gameinstance (cast `/Game/CoreElements/BP_MusicStones_Gameinstance` (`GameplayStatics.GetGameInstance`)))
  (set `self.As BP Music Stones Gameinstance` _asbp_music_stones_gameinstance))

(event `self.ReceiveActorBeginOverlap`
  (params (OtherActor :type "Actor Object Reference"))
  (set `self.Note_C_count` (+ 1.0 (`self.Note_C_count`))))

(fn `UserConstructionScript`)